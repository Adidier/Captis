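; Chicken actor that moves along a spline path and can be picked up and dropped by the VR motion controller.
; On BeginPlay, an active chicken randomly plays one of two timelines that map alpha to spline distance, with opposite 90-degree yaw offsets.
; Pickup stops path movement and physics to attach it; Drop detaches with physics on, without resuming movement.
; Overlapping a Door destroys it, except the first time if Start is set.
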(event OnComponentBeginOverlap(Sphere)
  (params (OverlappedComponent :type Primitive%20Component%20Object%20Reference) (OtherActor :type Actor%20Object%20Reference) (OtherComp :type Primitive%20Component%20Object%20Reference) (OtherBodyIndex :type Integer) (bFromSweep :type Boolean) (SweepResult :type Hit%20Result%20Structure%20%28by%20ref%29))
  (Utilities|Casting|CastToDoor OtherActor)
  (if (Variables|Default|GetStart)
    (Variables|Default|SetStart false)
    (else
      (Actor|DestroyActor))))

(event Custom|moveChicken
  (Components|Timeline|SetPlayRate (Variables|Default|GetTimeline_0) (/ 1.0 (Variables|Default|Getduration)))
  (Components|Timeline|SetNewTime (Variables|Default|GetTimeline_0) (Variables|Default|Getoffset))
  (if (> (Math|Random|RandomIntegerinRange 0 10) 5)
    (bind _transition (Timeline|Timeline_0 Play)
      (:Update
        (if (Variables|Default|GetActive)
          (Variables|Default|SetAlpha _transition)
          (Transformation|SetActorLocationAndRotation (Spline|GetLocationatDistanceAlongSpline (Variables|/Game/Blueprints/PathChicken.PathChicken_C|GetSpline (Variables|Default|GetPath)) (Math|Float|Lerp 0.0 (Spline|GetSplineLength (Variables|/Game/Blueprints/PathChicken.PathChicken_C|GetSpline (Variables|Default|GetPath))) (Variables|Default|GetAlpha)) "World") (Spline|GetRotationatDistanceAlongSpline (Variables|/Game/Blueprints/PathChicken.PathChicken_C|GetSpline (Variables|Default|GetPath)) (Math|Float|Lerp 0.0 (Spline|GetSplineLength (Variables|/Game/Blueprints/PathChicken.PathChicken_C|GetSpline (Variables|Default|GetPath))) (Variables|Default|GetAlpha)) "World"))
          (Transformation|AddActorLocalRotation "0,-90.000000, 0" false false))))
    (else
      (bind _transition_2 (Timeline|Timeline_1 Play)
        (:Update
          (if (Variables|Default|GetActive)
            (Variables|Default|SetAlpha _transition_2)
            (Transformation|SetActorLocationAndRotation (Spline|GetLocationatDistanceAlongSpline (Variables|/Game/Blueprints/PathChicken.PathChicken_C|GetSpline (Variables|Default|GetPath)) (Math|Float|Lerp 0.0 (Spline|GetSplineLength (Variables|/Game/Blueprints/PathChicken.PathChicken_C|GetSpline (Variables|Default|GetPath))) (Variables|Default|GetAlpha)) "World") (Spline|GetRotationatDistanceAlongSpline (Variables|/Game/Blueprints/PathChicken.PathChicken_C|GetSpline (Variables|Default|GetPath)) (Math|Float|Lerp 0.0 (Spline|GetSplineLength (Variables|/Game/Blueprints/PathChicken.PathChicken_C|GetSpline (Variables|Default|GetPath))) (Variables|Default|GetAlpha)) "World"))
            (Transformation|AddActorLocalRotation "0,90.000000,0.000000" false false)))))))

(event EventBeginPlay
  (if (Variables|Default|GetActive)
    (CallFunction|MoveChicken)))

(event Collision|EventActorBeginOverlap
  (params (OtherActor :type Actor%20Object%20Reference)))

(event EventTick
  (params (DeltaSeconds :type Float%20%28single-precision%29)))

(event EventPickup
  (params (AttachTo :type Scene%20Component%20Object%20Reference))
  (Development|PrintString "1")
  (Variables|Default|SetActive false)
  (Physics|SetSimulatePhysics (Variables|Default|Getchicken) false)
  (Transformation|AttachComponentToComponent (VehicleSound|GetRootComponent) AttachTo "None" "KeepWorld" "KeepWorld" "KeepWorld" false)
  (Development|PrintString "Hello"))

(event EventDrop
  (Physics|SetSimulatePhysics (Variables|Default|Getchicken) true)
  (Transformation|DetachFromActor "KeepWorld" "KeepWorld" "KeepWorld"))

(fn ConstructionScript)