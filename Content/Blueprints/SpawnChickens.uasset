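; Chicken spawner actor that creates a Chicken at the world origin about once per second and assigns it a path.
; BeginPlay caches every PathChicken actor in the level.
; Tick runs through a one-second Delay that throttles spawning.
; Each new chicken's Path comes from walking the cached list and stopping on a random roll, which favors earlier entries and falls back to the last.
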(event EventBeginPlay
  (bind _outactors (Actor|GetAllActorsOfClass "/Game/Blueprints/PathChicken.PathChicken_C"))
  (Variables|Default|Setpaths _outactors))

(event Collision|EventActorBeginOverlap
  (params (OtherActor :type Actor%20Object%20Reference)))

(event EventTick
  (params (DeltaSeconds :type Float%20%28single-precision%29))
  (Utilities|FlowControl|Delay 1.0)
  (bind _returnvalue (Game|SpawnActorfromClass "/Game/Blueprints/Chicken.Chicken_C" (Math|Conversions|ToTransform(Vector) (Math|Vector|MakeVector 0.0 0.0 0.0)) "Undefined" 0 0))
  (bind _array_element (Utilities|Array|ForEachLoopwithBreak (Variables|Default|Getpaths) :!label _label)
    (:LoopBody
      (if (> (Math|Random|RandomIntegerinRange 0 10) 5)
        (goto _label Break)))
    (:Completed
      (Variables|/Game/Blueprints/Chicken.Chicken_C|SetPath _returnvalue _array_element))))

(fn ConstructionScript)